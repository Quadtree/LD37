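; Player controller that shows the in-game HUD and handles leaving a finished match.
; On BeginPlay it creates the InGameUI widget and adds it to the viewport.
; Pressing Enter searches for existing WinDialog or LoseDialog widgets and, if either is found, loads the TitleScreen map.
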(event `self.ReceiveBeginPlay`
  (bind _returnvalue (`|CreateWidget` "/Game/UI/InGameUI.InGameUI_C"))
  (`UserWidget.AddToViewport` _returnvalue 0))

(event `self.ReceiveTick`
  (params (DeltaSeconds :type "Float (single-precision)")))

(event `Key|Enter` :paused true
  (params (Key :type "Key Structure" :default "AnyKey"))
  (:`Pressed`
    (bind _foundwidgets (`WidgetBlueprintLibrary.GetAllWidgetsOfClass` "/Game/UI/WinDialog.WinDialog_C" false))
    (bind _foundwidgets_2 (`WidgetBlueprintLibrary.GetAllWidgetsOfClass` "/Game/UI/LoseDialog.LoseDialog_C" false))
    (if (or (> (`KismetArrayLibrary.Array_Length` _foundwidgets) 0) (> (`KismetArrayLibrary.Array_Length` _foundwidgets_2) 0))
      (`GameplayStatics.OpenLevel` "/Game/Map/TitleScreen"))))

(fn `UserConstructionScript`)