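; Game mode Blueprint that plays battle music and decides when the match is won or lost.
; Every Tick it scans all Toybox actors and flags whether team 0 and the opposing team still have any.
; It shows a WinDialog when only team 0 remains, or a LoseDialog when team 0 has none.
; Nothing latches the result, so a new dialog widget is created each frame once the match ends.
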(event `self.ReceiveBeginPlay`
  (`GameplayStatics.PlaySound2D` "/Game/Sound/battle.battle" 0.5))

(event `self.ReceiveTick`
  (params (DeltaSeconds :type "Float (single-precision)"))
  (bind _outactors (`GameplayStatics.GetAllActorsOfClass` "/Script/LD37.Toybox"))
  (set `self.Team0Alive` false)
  (set `self.Team1Alive` false)
  (for _array_element _outactors
    (if (== (`Toybox.Team` _array_element) 0)
      (set `self.Team0Alive` true)
      (else
        (set `self.Team1Alive` true))))
  (if (`self.Team0Alive`)
    (if (not (`self.Team1Alive`))
      (bind _returnvalue (`|CreateWidget` "/Game/UI/WinDialog.WinDialog_C"))
      (`UserWidget.AddToViewport` _returnvalue 0))
    (else
      (bind _returnvalue_2 (`|CreateWidget` "/Game/UI/LoseDialog.LoseDialog_C"))
      (`UserWidget.AddToViewport` _returnvalue_2 0))))

(fn `UserConstructionScript`)